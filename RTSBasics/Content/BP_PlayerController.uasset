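; Player controller Blueprint that handles click selection of units under the cursor and tracks them in a SelectedUnits list.
; Pressing Select runs a Visibility trace under the cursor and, if the hit actor implements BPI_Unit, sends it SelectMessage.
; It then queries the unit's selection state through the interface, adding it uniquely to the list if selected and removing it otherwise.
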(event `InputAction|Select`
  (params (Key :type "Key Structure"))
  (bind (_hitresult _returnvalue) (`self.GetHitResultUnderCursorByChannel` "TraceTypeQuery1" false))
  (bind _selectedunits (`self.SelectedUnits`))
  (bind (_bblockinghit _binitialoverlap _time _distance _location _impactpoint _normal _impactnormal _physmat _hitactor) (`GameplayStatics.BreakHitResult` _hitresult))
  (:`Pressed`
    (if _returnvalue
      (if (`KismetSystemLibrary.DoesImplementInterface` _hitactor "/Game/TopDownCPP/Blueprints/BPI_Unit.BPI_Unit_C")
        (message `/Game/TopDownCPP/Blueprints/BPI_Unit.Select` _hitactor)
        (bind _bselected (message `/Game/TopDownCPP/Blueprints/BPI_Unit.IsSelected` _hitactor))
        (if _bselected
          (`KismetArrayLibrary.Array_AddUnique` _selectedunits _hitactor)
          (else
            (`KismetArrayLibrary.Array_RemoveItem` _selectedunits _hitactor)))))))

(fn `UserConstructionScript`)